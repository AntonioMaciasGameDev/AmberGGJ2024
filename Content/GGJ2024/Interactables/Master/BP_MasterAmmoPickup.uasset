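; BP_MasterAmmoPickup is an ammo pickup, named as a master class, that tops up the player's gun, rifle or shotgun ammo on interaction.
; InteractInterface checks the passed Alan reference, then AddAmmo switches on WeaponName to one add function per weapon and destroys the actor.
; Each function adds AmmoAmount through the stored AsBPAlan variable, which this graph never sets, and prints the new total on screen.
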(event `/Game/GGJ2024/Interfaces/BPI_Interact.Interact Interface`
  (params (AlanRef :type "/Game/GGJ2024/Player/BP_Alan Object Reference"))
  (`/Engine/EditorBlueprintResources/StandardMacros.IsValid` AlanRef
    (:`Is Valid`
      (`KismetSystemLibrary.PrintString` "Hello")
      (`self.AddAmmo`))))

(event `AddAmmo`
  (switch `/Game/GGJ2024/Guns/E_WeaponName` (`self.WeaponName`)
    (:`NewEnumerator0`
      (`self.Add Gun Ammo`))
    (:`NewEnumerator1`
      (`self.Add Rifle Ammo`))
    (:`NewEnumerator2`
      (`self.Add Shotgun Ammo`)))
  (`self.K2_DestroyActor`))

(fn `Add Gun Ammo`
  (bind _as_bp_alan (`self.As BP Alan`))
  (bind _output_get (set `/Game/GGJ2024/Player/BP_Alan.GunAmmo` (+ (`/Game/GGJ2024/Player/BP_Alan.GunAmmo` _as_bp_alan) (`self.Ammo Amount`)) _as_bp_alan))
  (`KismetSystemLibrary.PrintString` (`KismetStringLibrary.Concat_StrStr` "Added " " " (`KismetStringLibrary.Conv_IntToString` _output_get) " " "*Gun* Ammo") true true (struct :`R` 1.0 :`G` 0.77448 :`A` 1.0) 5.0))

(fn `Add Rifle Ammo`
  (bind _as_bp_alan (`self.As BP Alan`))
  (bind _output_get (set `/Game/GGJ2024/Player/BP_Alan.RifleAmmo` (+ (`/Game/GGJ2024/Player/BP_Alan.RifleAmmo` _as_bp_alan) (`self.Ammo Amount`)) _as_bp_alan))
  (`KismetSystemLibrary.PrintString` (`KismetStringLibrary.Concat_StrStr` "Added " " " (`KismetStringLibrary.Conv_IntToString` _output_get) " " "*Rifle* Ammo") true true (struct :`R` 1.0 :`G` 0.77448 :`A` 1.0) 5.0))

(fn `Add Shotgun Ammo`
  (bind _as_bp_alan (`self.As BP Alan`))
  (bind _output_get (set `/Game/GGJ2024/Player/BP_Alan.ShotgunAmmo` (+ (`/Game/GGJ2024/Player/BP_Alan.ShotgunAmmo` _as_bp_alan) (`self.Ammo Amount`)) _as_bp_alan))
  (`KismetSystemLibrary.PrintString` (`KismetStringLibrary.Concat_StrStr` "Added " " " (`KismetStringLibrary.Conv_IntToString` _output_get) " " "*Shotgun* Ammo") true true (struct :`R` 1.0 :`G` 0.77448 :`A` 1.0) 5.0))

(fn `UserConstructionScript`
  (`parent.UserConstructionScript`))