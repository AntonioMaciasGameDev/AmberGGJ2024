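; BP_MasterPickupWeapon is a master pickup Blueprint that gives a weapon to the interacting character.
; Its Interact event runs the parent logic, then calls SpawnWeapon on the passed Alan reference with the configured WeaponToSpawn.
; The construction script fills the SItems item struct, converting the WeaponName enum to a name.
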(event `/Game/GGJ2024/Interfaces/BPI_Interact.Interact`
  (params (`Alan Ref` :type "/Game/GGJ2024/Player/BP_Alan Object Reference"))
  (`parent.Interact` `Alan Ref`)
  (`/Game/GGJ2024/Player/BP_Alan.SpawnWeapon` `Alan Ref` (`self.WeaponToSpawn`)))

(fn `UserConstructionScript`
  (`parent.UserConstructionScript`)
  (set `self.S_Items` (make `/Game/GGJ2024/Player/Inventory/S_Items` (`|GetEnumeratorName` (`self.WeaponName`)) null null)))