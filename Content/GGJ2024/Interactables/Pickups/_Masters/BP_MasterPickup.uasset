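; BP_MasterPickup is a pickup Blueprint, named as a master class, for items that go into the inventory of the player character, BP_Alan.
; BeginPlay casts and caches the player character, and the IA_Interact input action passes SItems to its AddToInventoryMessage.
; Separately, the Interact event checks the Alan reference it receives and calls Destroy, which removes the actor after a short delay.
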(event `self.ReceiveBeginPlay`
  (bind _asbp_alan (cast `/Game/GGJ2024/Player/BP_Alan` (`GameplayStatics.GetPlayerCharacter` 0)))
  (set `self.As BP Alan` _asbp_alan))

(event `Destroy`
  (`KismetSystemLibrary.Delay` 0.1)
  (`self.K2_DestroyActor`))

(event `/Game/GGJ2024/Interfaces/BPI_Interact.Interact`
  (params (`Alan Ref` :type "/Game/GGJ2024/Player/BP_Alan Object Reference"))
  (`/Engine/EditorBlueprintResources/StandardMacros.IsValid` `Alan Ref`
    (:`Is Valid`
      (`self.Destroy`))))

(event `EnhancedInput|/Game/GGJ2024/Player/Inputs/Actions/IA_Interact`
  (params (ActionValue :type Boolean) (ElapsedSeconds :type "Float (double-precision)") (TriggeredSeconds :type "Float (double-precision)") (InputAction :type "InputAction Object Reference" :default "/Game/GGJ2024/Player/Inputs/Actions/IA_Interact.IA_Interact"))
  (:`Started`
    (message `/Game/GGJ2024/Interfaces/BPI_Inventory.Add to Inventory` (`self.As BP Alan`) (`self.S_Items`))))

(fn `UserConstructionScript`)