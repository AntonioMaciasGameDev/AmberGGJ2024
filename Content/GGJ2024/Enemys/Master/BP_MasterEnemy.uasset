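; Master enemy character Blueprint that tracks health and takes damage, with double damage for weapon hits to the head.
; The construction script fills health from MaxHealth, and BeginPlay caches the player as BP_Alan.
; HeadCollision overlaps with a BP_MasterWeapon apply twice that weapon's damage to the enemy.
; AnyDamage subtracts health, halts movement immediately and prints debug text; no death handling is present here.
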(event `self.ReceiveBeginPlay`
  (bind _asbp_alan (cast `/Game/GGJ2024/Player/BP_Alan` (`GameplayStatics.GetPlayerCharacter` 0)))
  (set `self.As BP Alan` _asbp_alan))

(event `self.ReceiveAnyDamage`
  (params (Damage :type "Float (single-precision)") (DamageType :type "DamageType Object Reference") (InstigatedBy :type "Controller Object Reference") (DamageCauser :type "Actor Object Reference"))
  (bind _output_get (set `self.Healt` (- (`self.Healt`) Damage)))
  (`MovementComponent.StopMovementImmediately` (`self.CharacterMovement`))
  (`KismetSystemLibrary.PrintString` (`KismetStringLibrary.Concat_StrStr` (`KismetStringLibrary.Conv_DoubleToString` Damage) " " "Damage recived" " " "Current health" " " (`KismetStringLibrary.Conv_DoubleToString` _output_get)) true true (struct :`R` 1.0 :`G` 0.407668 :`B` 0.185832 :`A` 1.0)))

(event `self.HeadCollision.OnComponentBeginOverlap`
  (params (OverlappedComponent :type "PrimitiveComponent Object Reference") (OtherActor :type "Actor Object Reference") (OtherComp :type "PrimitiveComponent Object Reference") (OtherBodyIndex :type Integer) (bFromSweep :type Boolean) (SweepResult :type "HitResult Structure (by ref)"))
  (bind _asbp_master_weapon (cast `/Game/GGJ2024/Guns/Master/BP_MasterWeapon` OtherActor))
  (`GameplayStatics.ApplyDamage` self (* (`/Game/GGJ2024/Guns/Master/BP_MasterWeapon.Damage` _asbp_master_weapon) 2.0) null _asbp_master_weapon)
  (`KismetSystemLibrary.PrintString` "HeadShot"))

(fn `UserConstructionScript`
  (set `self.Healt` (`self.MaxHealth`)))