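; BP_SuicideEnemy is an enemy that rushes the player and deals area damage before destroying itself.
; When its PawnSensing component sees any pawn, it calls FollowPawn, which uses AI MoveTo to chase player character 0.
; On reaching the acceptance radius, it applies full radial damage around itself from its Damage variable, then destroys itself after a short delay.
; A failed move has no handling.
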(event `self.PawnSensing.OnSeePawn`
  (params (Pawn :type "Pawn Object Reference"))
  (`self.Follow Pawn`))

(event `Follow Pawn`
  (`|AIMoveTo` self (0.0 0.0 0.0) (`GameplayStatics.GetPlayerCharacter` 0) 250.0
    (:`OnSuccess`
      (`GameplayStatics.ApplyRadialDamage` :`BaseDamage` (`self.Damage`) :`Origin` (`self.K2_GetActorLocation`) :`DamageRadius` 300.0 :`DamageCauser` self :`InstigatedByController` null :`bDoFullDamage` true)
      (`KismetSystemLibrary.Delay` 0.5)
      (`self.K2_DestroyActor`))))

(fn `UserConstructionScript`)